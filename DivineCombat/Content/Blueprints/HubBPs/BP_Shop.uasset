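; BP_Shop is a hub shop trigger that shows the W_Shop widget while its Box is overlapped.
; Begin overlap creates a new widget, adds it to the viewport and shows the mouse cursor; end overlap removes the widget but leaves the cursor visible.
; Both events cast player character 0 to BP_PlayerAvatar rather than checking the overlapping actor.
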(event `self.Box.OnComponentBeginOverlap`
  (params (OverlappedComponent :type "PrimitiveComponent Object Reference") (OtherActor :type "Actor Object Reference") (OtherComp :type "PrimitiveComponent Object Reference") (OtherBodyIndex :type Integer) (bFromSweep :type Boolean) (SweepResult :type "HitResult Structure (by ref)"))
  (cast `/Game/Blueprints/HubBPs/HubUnits/BP_PlayerAvatar` (`GameplayStatics.GetPlayerCharacter` 0))
  (bind _returnvalue (`|CreateWidget` "/Game/Blueprints/UI_Widgets/WIP_UI/Inventory/InventorySystem-Advanced/UI/W_Shop.W_Shop_C"))
  (`UserWidget.AddToViewport` _returnvalue 0)
  (bind _asplayer_controller (cast `PlayerController` (`GameplayStatics.GetPlayerController` 0)))
  (set `PlayerController.bShowMouseCursor` true _asplayer_controller))

(event `self.Box.OnComponentEndOverlap`
  (params (OverlappedComponent :type "PrimitiveComponent Object Reference") (OtherActor :type "Actor Object Reference") (OtherComp :type "PrimitiveComponent Object Reference") (OtherBodyIndex :type Integer))
  (cast `/Game/Blueprints/HubBPs/HubUnits/BP_PlayerAvatar` (`GameplayStatics.GetPlayerCharacter` 0))
  (`Widget.RemoveFromParent` (stale `self.Box.OnComponentBeginOverlap` _returnvalue)))

(fn `UserConstructionScript`)