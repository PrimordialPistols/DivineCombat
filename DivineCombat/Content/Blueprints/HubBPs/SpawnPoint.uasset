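; Hub spawn point that spawns a deity or hero hub actor at its own transform when the game stage matches the stage assigned to it.
; On BeginPlay it reads Stage and DeityToSpawn from BP_MyGameInstance.
; Only stages 2 and 3 spawn anything, through duplicated branches that pick the Mel, Aelia, Aevum or Hero hub class and adjust for collisions but always spawn.
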(event `self.ReceiveBeginPlay`
  (bind _returnvalue (`self.GetTransform`))
  (bind _returnvalue_2 (`self.GetTransform`))
  (bind _asbp_my_game_instance (cast `/Game/Blueprints/SaveSystem/BP_MyGameInstance` (`GameplayStatics.GetGameInstance`)))
  (if (== (`/Game/Blueprints/SaveSystem/BP_MyGameInstance.Stage` _asbp_my_game_instance) 2)
    (if (== (`self.StageForSpawnPoint `) 2)
      (bind _deitytospawn (`/Game/Blueprints/SaveSystem/BP_MyGameInstance.DeityToSpawn` _asbp_my_game_instance))
      (switch `/Game/DataStructures/Enum_Divine` _deitytospawn
        (:`NewEnumerator0`
          (`|SpawnActorFromClass` (`self.MelHub`) _returnvalue_2 "AdjustIfPossibleButAlwaysSpawn" "OverrideRootScale" null null))
        (:`NewEnumerator1`
          (`|SpawnActorFromClass` (`self.AeliaHub`) _returnvalue_2 "AdjustIfPossibleButAlwaysSpawn" "OverrideRootScale" null null))
        (:`NewEnumerator2`
          (`|SpawnActorFromClass` (`self.AevumHub`) _returnvalue_2 "AdjustIfPossibleButAlwaysSpawn" "OverrideRootScale" null null))
        (:`NewEnumerator3`
          (`|SpawnActorFromClass` (`self.HeroHub`) _returnvalue_2 "AdjustIfPossibleButAlwaysSpawn" "OverrideRootScale" null null))))
    (elif (== (`/Game/Blueprints/SaveSystem/BP_MyGameInstance.Stage` _asbp_my_game_instance) 3)
      (if (== (`self.StageForSpawnPoint `) 3)
        (switch `/Game/DataStructures/Enum_Divine` _deitytospawn
          (:`NewEnumerator0`
            (`|SpawnActorFromClass` (`self.MelHub`) _returnvalue "AdjustIfPossibleButAlwaysSpawn" "OverrideRootScale" null null))
          (:`NewEnumerator1`
            (`|SpawnActorFromClass` (`self.AeliaHub`) _returnvalue "AdjustIfPossibleButAlwaysSpawn" "OverrideRootScale" null null))
          (:`NewEnumerator2`
            (`|SpawnActorFromClass` (`self.AevumHub`) _returnvalue "AdjustIfPossibleButAlwaysSpawn" "OverrideRootScale" null null))
          (:`NewEnumerator3`
            (`|SpawnActorFromClass` (`self.HeroHub`) _returnvalue "AdjustIfPossibleButAlwaysSpawn" "OverrideRootScale" null null)))))))

(fn `UserConstructionScript`)