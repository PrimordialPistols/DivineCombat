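; BP_TrainingGround is a hub actor that opens the unit upgrade menu through a Box overlap trigger.
; Begin overlap compares the overlapped component to BP_PlayerAvatar, then creates W_UnitUpgradeMenu, shows the mouse cursor and sets Game and UI input focused on it.
; End overlap checks only that the player character is BP_PlayerAvatar, then removes the widget without restoring cursor or input mode.
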(event `self.Box.OnComponentBeginOverlap`
  (params (OverlappedComponent :type "PrimitiveComponent Object Reference") (OtherActor :type "Actor Object Reference") (OtherComp :type "PrimitiveComponent Object Reference") (OtherBodyIndex :type Integer) (bFromSweep :type Boolean) (SweepResult :type "HitResult Structure (by ref)"))
  (bind _returnvalue (`GameplayStatics.GetPlayerController` 0))
  (if (== OverlappedComponent "/Game/Blueprints/HubBPs/HubUnits/BP_PlayerAvatar.BP_PlayerAvatar")
    (cast `/Game/Blueprints/HubBPs/HubUnits/BP_PlayerAvatar` (`GameplayStatics.GetPlayerCharacter` 0))
    (bind _returnvalue_2 (`|CreateWidget` "/Game/Blueprints/UI_Widgets/IngameMenus/UnitTrainingMenu/W_UnitUpgradeMenu.W_UnitUpgradeMenu_C"))
    (`UserWidget.AddToViewport` _returnvalue_2 0)
    (bind _asplayer_controller (cast `PlayerController` _returnvalue))
    (set `PlayerController.bShowMouseCursor` true _asplayer_controller)
    (`WidgetBlueprintLibrary.SetInputMode_GameAndUIEx` _returnvalue _returnvalue_2)))

(event `self.Box.OnComponentEndOverlap`
  (params (OverlappedComponent :type "PrimitiveComponent Object Reference") (OtherActor :type "Actor Object Reference") (OtherComp :type "PrimitiveComponent Object Reference") (OtherBodyIndex :type Integer))
  (cast `/Game/Blueprints/HubBPs/HubUnits/BP_PlayerAvatar` (`GameplayStatics.GetPlayerCharacter` 0))
  (`Widget.RemoveFromParent` (stale `self.Box.OnComponentBeginOverlap` _returnvalue_2)))

(fn `UserConstructionScript`)