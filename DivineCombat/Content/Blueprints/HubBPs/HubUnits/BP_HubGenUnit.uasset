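; Generic hub unit actor whose look depends on its class and the deity choice stored in the game instance.
; The construction script sets an axe, spear, sword or archer skeletal mesh from UnitType, then reads DeityChoice from BP_MyGameInstance.
; A value of 1 or above swaps lapel, helmet fur and cape materials to one of two variants; lower values keep the mesh's materials.
; The event graph holds no logic.
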(fn `UserConstructionScript`
  (bind _skeletalmesh (`self.SkeletalMesh`))
  (bind _skeletalmesh_2 (`self.SkeletalMesh`))
  (bind _skeletalmesh_3 (`self.SkeletalMesh`))
  (bind _skeletalmesh_4 (`self.SkeletalMesh`))
  (bind _skeletalmesh_5 (`self.SkeletalMesh`))
  (bind _skeletalmesh_6 (`self.SkeletalMesh`))
  (bind _skeletalmesh_7 (`self.SkeletalMesh`))
  (bind _skeletalmesh_8 (`self.SkeletalMesh`))
  (bind _skeletalmesh_9 (`self.SkeletalMesh`))
  (switch `/Game/DataStructures/Enum_UnitClass` (`self.UnitType`)
    (:`NewEnumerator0`
      (`SkinnedMeshComponent.SetSkinnedAssetAndUpdate` _skeletalmesh_8 "/Game/3DArtAssets/CharacterModels/GenericUnits/AxeUnit/GenAxeUnitSkeletalMesh.GenAxeUnitSkeletalMesh" true))
    (:`NewEnumerator1`
      (`SkinnedMeshComponent.SetSkinnedAssetAndUpdate` _skeletalmesh_8 "/Game/3DArtAssets/CharacterModels/GenericUnits/SpearUnit/New/GenSpearUnitSkeletalMesh.GenSpearUnitSkeletalMesh" true))
    (:`NewEnumerator2`
      (`SkinnedMeshComponent.SetSkinnedAssetAndUpdate` _skeletalmesh_8 "/Game/3DArtAssets/CharacterModels/GenericUnits/SwordUnit/GenSwordUnitSkeletalMesh.GenSwordUnitSkeletalMesh" true))
    (:`NewEnumerator3`
      (`SkinnedMeshComponent.SetSkinnedAssetAndUpdate` _skeletalmesh_8 "/Game/3DArtAssets/CharacterModels/GenericUnits/ArcherUnit/GenArcherUnitSkeletalMesh.GenArcherUnitSkeletalMesh" true)))
  (bind _asbp_my_game_instance (cast `/Game/Blueprints/SaveSystem/BP_MyGameInstance` (`GameplayStatics.GetGameInstance`)))
  (`/Engine/EditorBlueprintResources/StandardMacros.CompareInt` (`/Game/Blueprints/SaveSystem/BP_MyGameInstance.DeityChoice` _asbp_my_game_instance) 1
    (:`>`
      (switch `/Game/DataStructures/Enum_UnitClass` (`self.UnitType`)
        (:`NewEnumerator0`
          (`PrimitiveComponent.SetMaterial` _skeletalmesh 0 "/Game/3DArtAssets/CharacterModels/GenericUnits/AxeUnit/Textures/Mel/GenAxUnit_M_Lapel_MAT.GenAxUnit_M_Lapel_MAT")
          (`PrimitiveComponent.SetMaterial` _skeletalmesh 4 "/Game/3DArtAssets/CharacterModels/GenericUnits/AxeUnit/Textures/Mel/GenAxUnit_M_HelmetFur_MAT.GenAxUnit_M_HelmetFur_MAT")
          (`PrimitiveComponent.SetMaterial` _skeletalmesh 7 "/Game/3DArtAssets/CharacterModels/GenericUnits/AxeUnit/Textures/Mel/GenAxUnit_M_Cape_MAT.GenAxUnit_M_Cape_MAT"))
        (:`NewEnumerator1`
          (`PrimitiveComponent.SetMaterial` _skeletalmesh_2 4 "/Game/3DArtAssets/CharacterModels/GenericUnits/SpearUnit/Textures/Mel/GenSpUnit_M_HelmetFur_MAT.GenSpUnit_M_HelmetFur_MAT")
          (`PrimitiveComponent.SetMaterial` _skeletalmesh_2 5 "/Game/3DArtAssets/CharacterModels/GenericUnits/SpearUnit/Textures/Mel/GenSpUnit_M_Lapel_MAT.GenSpUnit_M_Lapel_MAT")
          (`PrimitiveComponent.SetMaterial` _skeletalmesh_2 9 "/Game/3DArtAssets/CharacterModels/GenericUnits/SpearUnit/Textures/Mel/GenSpUnit_M_Cape_MAT.GenSpUnit_M_Cape_MAT"))
        (:`NewEnumerator2`
          (`PrimitiveComponent.SetMaterial` _skeletalmesh_3 3 "/Game/3DArtAssets/CharacterModels/GenericUnits/SwordUnit/Textures/Mel/GenSwUnit_M_HelmetFur_MAT.GenSwUnit_M_HelmetFur_MAT")
          (`PrimitiveComponent.SetMaterial` _skeletalmesh_3 7 "/Game/3DArtAssets/CharacterModels/GenericUnits/SwordUnit/Textures/Mel/GenSwUnit_M_Lapel_MAT.GenSwUnit_M_Lapel_MAT")
          (`PrimitiveComponent.SetMaterial` _skeletalmesh_3 9 "/Game/3DArtAssets/CharacterModels/GenericUnits/SwordUnit/Textures/Mel/GenSwUnit_M_Cape_MAT.GenSwUnit_M_Cape_MAT"))
        (:`NewEnumerator3`
          (`PrimitiveComponent.SetMaterial` _skeletalmesh_9 1 "/Game/3DArtAssets/CharacterModels/GenericUnits/ArcherUnit/Textures/Mel/GenArUnit_M_Lapel.GenArUnit_M_Lapel")
          (`PrimitiveComponent.SetMaterial` _skeletalmesh_9 4 "/Game/3DArtAssets/CharacterModels/GenericUnits/ArcherUnit/Textures/Mel/GenArUnit_M_Cape_MAT.GenArUnit_M_Cape_MAT")
          (`PrimitiveComponent.SetMaterial` _skeletalmesh_9 9 "/Game/3DArtAssets/CharacterModels/GenericUnits/ArcherUnit/Textures/Mel/GenArUnit_M_HelmetFur_MAT.GenArUnit_M_HelmetFur_MAT"))))
    (:`==`
      (switch `/Game/DataStructures/Enum_UnitClass` (`self.UnitType`)
        (:`NewEnumerator0`
          (`PrimitiveComponent.SetMaterial` _skeletalmesh_4 0 "/Game/3DArtAssets/CharacterModels/GenericUnits/AxeUnit/Textures/Aelia/GenAxUnit_A_Lapel_MAT.GenAxUnit_A_Lapel_MAT")
          (`PrimitiveComponent.SetMaterial` _skeletalmesh_4 4 "/Game/3DArtAssets/CharacterModels/GenericUnits/AxeUnit/Textures/Aelia/GenAxUnit_A_HelmetFur_MAT.GenAxUnit_A_HelmetFur_MAT")
          (`PrimitiveComponent.SetMaterial` _skeletalmesh_4 7 "/Game/3DArtAssets/CharacterModels/GenericUnits/AxeUnit/Textures/Aelia/GenAxUnit_A_Cape_MAT.GenAxUnit_A_Cape_MAT"))
        (:`NewEnumerator1`
          (`PrimitiveComponent.SetMaterial` _skeletalmesh_5 4 "/Game/3DArtAssets/CharacterModels/GenericUnits/SpearUnit/Textures/Aelia/GenSpUnit_A_HelmetFur_MAT.GenSpUnit_A_HelmetFur_MAT")
          (`PrimitiveComponent.SetMaterial` _skeletalmesh_5 5 "/Game/3DArtAssets/CharacterModels/GenericUnits/SpearUnit/Textures/Aelia/GenSpUnit_A_Lapel_MAT.GenSpUnit_A_Lapel_MAT")
          (`PrimitiveComponent.SetMaterial` _skeletalmesh_5 9 "/Game/3DArtAssets/CharacterModels/GenericUnits/SpearUnit/Textures/Aelia/GenSpUnit_A_Cape_MAT.GenSpUnit_A_Cape_MAT"))
        (:`NewEnumerator2`
          (`PrimitiveComponent.SetMaterial` _skeletalmesh_6 3 "/Game/3DArtAssets/CharacterModels/GenericUnits/SwordUnit/Textures/Aelia/GenSwUnit_A_HelmetFur_MAT.GenSwUnit_A_HelmetFur_MAT")
          (`PrimitiveComponent.SetMaterial` _skeletalmesh_6 7 "/Game/3DArtAssets/CharacterModels/GenericUnits/SwordUnit/Textures/Aelia/GenSwUnit_A_Lapel_MAT.GenSwUnit_A_Lapel_MAT")
          (`PrimitiveComponent.SetMaterial` _skeletalmesh_6 9 "/Game/3DArtAssets/CharacterModels/GenericUnits/SwordUnit/Textures/Aelia/GenSwUnit_A_Cape_MAT.GenSwUnit_A_Cape_MAT"))
        (:`NewEnumerator3`
          (`PrimitiveComponent.SetMaterial` _skeletalmesh_7 1 "/Game/3DArtAssets/CharacterModels/GenericUnits/ArcherUnit/Textures/Aelia/GenArUnit_A_Lapel_MAT.GenArUnit_A_Lapel_MAT")
          (`PrimitiveComponent.SetMaterial` _skeletalmesh_7 4 "/Game/3DArtAssets/CharacterModels/GenericUnits/ArcherUnit/Textures/Aelia/GenArUnit_A_Cape_MAT.GenArUnit_A_Cape_MAT")
          (`PrimitiveComponent.SetMaterial` _skeletalmesh_7 9 "/Game/3DArtAssets/CharacterModels/GenericUnits/ArcherUnit/Textures/Aelia/GenArUnit_A_HelmetFur_MAT.GenArUnit_A_HelmetFur_MAT"))))))