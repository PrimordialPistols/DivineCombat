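; Game instance that manages a single save slot for the grid's goal tracker data.
; On Init it caches the first BP_Grid, then loads or creates a MySaveGame, starting a looping autosave timer only when a save already exists.
; Saving copies the grid's trackers into GoalTracker and writes SaveGameData, without visibly transferring them into it.
; LoadPlayerData makes the same grid-to-variable copy, and ClearData deletes the slot.
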(event `self.ReceiveInit`
  (bind _outactors (`GameplayStatics.GetAllActorsOfClass` "/Game/Blueprints/Grid/BP_Grid.BP_Grid_C"))
  (set `self.Grid Object` (`|GetArrayItem` _outactors))
  ;[1 1 1] Checks if save file exists
  (bind _returnvalue (`GameplayStatics.DoesSaveGameExist` (`self.SaveFileName`)))
  (if _returnvalue
    ;[1 1 1] Loads Save game data
    (bind _returnvalue_2 (`GameplayStatics.LoadGameFromSlot` (`self.SaveFileName`)))
    (bind _asmy_save_game (cast `/Game/Blueprints/Save/MySaveGame` _returnvalue_2))
    (set `self.SaveGameData` _asmy_save_game)
    (`KismetSystemLibrary.K2_SetTimer` self "AutoSaveData" 10.0 true)
    (`KismetSystemLibrary.PrintString` "Saved" true true (struct :`R` 0.747282 :`G` 1.0 :`A` 1.0))
    (else
      ;[1 1 1] If no game data exists creates save data
      (bind _returnvalue_3 (`GameplayStatics.CreateSaveGameObject` "/Game/Blueprints/Save/MySaveGame.MySaveGame_C"))
      (set `self.SaveGameData` _returnvalue_3)
      (`KismetSystemLibrary.PrintString` "Save data created" true true (struct :`R` 0.759106 :`G` 1.0 :`A` 1.0)))))

(fn `AutoSaveData`
  (`self.SavePlayerData`))

(fn `ClearData`
  (`GameplayStatics.DeleteGameInSlot` (`self.SaveFileName`)))

(fn `LoadPlayerData`
  (locals (GridRef :type "/Game/Blueprints/Grid/BP_Grid Object Reference") (`Goal tracker` :type "Array of /Game/Blueprints/Grid/Struct_GoalTrackers Structure"))
  (bind _asbp_grid (cast `/Game/Blueprints/Grid/BP_Grid` (`self.Grid Object`))
    (:`then`
      (bind _output_get (set `local.GridRef` _asbp_grid))
      (set `local.Goal tracker` (`/Game/Blueprints/Grid/BP_Grid.GoalTrackersStructs` _output_get)))
    (:`CastFailed`
      (`KismetSystemLibrary.PrintString` "Load Failed"))))

(fn `SavePlayerData`
  (locals (GridRef :type "/Game/Blueprints/Grid/BP_Grid Object Reference") (`Goal Tracker` :type "Array of /Game/Blueprints/Grid/Struct_GoalTrackers Structure"))
  (bind _asbp_grid (cast `/Game/Blueprints/Grid/BP_Grid` (`self.Grid Object`))
    (:`then`
      (bind _output_get (set `local.GridRef` _asbp_grid))
      (set `local.Goal Tracker` (`/Game/Blueprints/Grid/BP_Grid.GoalTrackersStructs` _output_get))
      (`GameplayStatics.SaveGameToSlot` (`self.SaveGameData`) (`self.SaveFileName`))
      (`KismetSystemLibrary.PrintString` "saved data" true true (struct :`R` 0.616475 :`G` 1.0 :`A` 1.0)))
    (:`CastFailed`
      (`KismetSystemLibrary.PrintString` "Save Failed"))))