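; Game mode for turn-based grid combat that sets up the combat screen, grid and starting unit list.
; BeginPlay creates W_CombatScreen, links it to the level's BP_Grid, then enables the spawn zone and damage tiles.
; FinishWorldSetup drops Divine units, orders the rest player-faction first for the screen, tallies both sides on the grid and hands over the player controller.
; Sorting assumes two factions; an insertion-sort version is left unconnected.
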(event `self.ReceiveBeginPlay`
  (bind _returnvalue (`|CreateWidget` "/Game/Blueprints/UI_Widgets/Combat/W_CombatScreen.W_CombatScreen_C"))
  (bind _output_get (set `self.CombatScreen` _returnvalue))
  (`UserWidget.AddToPlayerScreen` _output_get 0)
  ;[1 1 1] Get Local Reference to Grid
  (bind _outactors (`GameplayStatics.GetAllActorsOfClass` "/Game/Blueprints/GridBPs/GridObjects/BP_Grid.BP_Grid_C"))
  (bind _output_get_2 (set `self.grid` (`|GetArrayItem` _outactors)))
  (set `/Game/Blueprints/UI_Widgets/Combat/W_CombatScreen.grid` _output_get_2 (`self.CombatScreen`))
  (`/Game/Blueprints/GridBPs/GridObjects/BP_Grid.EnableSpawnZone` (`self.grid`))
  (`/Game/Blueprints/GridBPs/GridObjects/BP_Grid.ActivateDamageTiles` (`self.grid`)))

(event `FinishWorldSetup`
  (bind _grid (`self.grid`))
  (bind _grid_2 (`self.grid`))
  ;[1 1 1] Create Unit List
  (bind _outactors (`GameplayStatics.GetAllActorsOfClass` "/Game/Blueprints/GridBPs/GridUnits/BP_Unit.BP_Unit_C"))
  (bind _notdivineunits (`self.CheckIfDivine` _outactors)) ; Checks if unit is divine if not add to list
  (bind _sortedunits (`self.SortUnitListByFaction` _notdivineunits)) ; Currently only works for two factions, player and other
  (bind _output_get (set `/Game/Blueprints/UI_Widgets/Combat/W_CombatScreen.UnitList` _sortedunits (`self.CombatScreen`)))
  (for _array_element _output_get
    (if (`|EnumEquality` (`/Game/Blueprints/GridBPs/GridUnits/BP_Unit.UnitFaction` _array_element) "NewEnumerator0")
      (set `/Game/Blueprints/GridBPs/GridObjects/BP_Grid.StartingAlliedUnits` (+ (`/Game/Blueprints/GridBPs/GridObjects/BP_Grid.StartingAlliedUnits` _grid_2) 1) _grid_2)
      (else
        (set `/Game/Blueprints/GridBPs/GridObjects/BP_Grid.StartingEnemyUnits` (+ (`/Game/Blueprints/GridBPs/GridObjects/BP_Grid.StartingEnemyUnits` _grid) 1) _grid))))
  ;[1 1 1] Get Local Reference to HUD widget and PlayerController
  (set `/Game/Blueprints/UI_Widgets/Combat/W_CombatScreen.Player` (cast `/Game/Blueprints/Controllers/BP_PlayerController` (`GameplayStatics.GetPlayerController` 0) :!pure true) (`self.CombatScreen`)))

(fn `CheckIfDivine`
  (params (Units :type "Array of /Game/Blueprints/GridBPs/GridUnits/BP_Unit Object Reference"))
  (returns (NotDivineUnits :type "Array of /Game/Blueprints/GridBPs/GridUnits/BP_Unit Object Reference"))
  (locals (NonDivineUnits :type "Array of /Game/Blueprints/GridBPs/GridUnits/BP_Unit Object Reference"))
  ;[1 1 1] Checks if the Unit is divine if not will add them to a list to be sorted
  (for _array_element Units
    (if (not (`/Game/Blueprints/GridBPs/GridUnits/BP_Unit.UnitType_Divine` _array_element))
      (`KismetArrayLibrary.Array_Add` (`local.NonDivineUnits`) _array_element)))
  (return (`local.NonDivineUnits`)))

(fn `SortUnitListByFaction`
  (params (unsortedUnits :type "Array of /Game/Blueprints/GridBPs/GridUnits/BP_Unit Object Reference"))
  (returns (sortedUnits :type "Array of /Game/Blueprints/GridBPs/GridUnits/BP_Unit Object Reference"))
  (locals (sortingList :type "Array of /Game/Blueprints/GridBPs/GridUnits/BP_Unit Object Reference") (currentTarget :type "/Game/Blueprints/GridBPs/GridUnits/BP_Unit Object Reference") (currentTargetStepper :type Integer :default 1) (currentTargetFaction :type Integer :default 0) (playerFacList :type "Array of /Game/Blueprints/GridBPs/GridUnits/BP_Unit Object Reference") (enemyFacList :type "Array of /Game/Blueprints/GridBPs/GridUnits/BP_Unit Object Reference"))
  (for _array_element unsortedUnits
    (if (`|EnumEquality` (`/Game/Blueprints/GridBPs/GridUnits/BP_Unit.UnitFaction` _array_element) "NewEnumerator0")
      (`KismetArrayLibrary.Array_Add` (`local.playerFacList`) _array_element)
      (else
        (`KismetArrayLibrary.Array_Add` (`local.enemyFacList`) _array_element))))
  (for _array_element_2 (`local.enemyFacList`)
    (`KismetArrayLibrary.Array_Add` (`local.playerFacList`) _array_element_2))
  (return (`local.playerFacList`)))

(fn `UserConstructionScript`)