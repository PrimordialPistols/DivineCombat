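; Behavior tree task that asks a question in the dialogue UI and waits for the player to pick a response.
; It gets the DB_Daius dialogue box from the blackboard, sets its text and fills a response options overlay with one clickable widget per response.
; Each click delegate is bound to an event, and ResponseReceived stores the answer in the blackboard as a string, removes the options and finishes the task successfully.
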(event `self.ReceiveExecuteAI`
  (params (OwnerController :type "AIController Object Reference") (ControlledPawn :type "Pawn Object Reference"))
  (bind _asdb_daius (cast `/Game/Blueprints/UI_Widgets/NPCDialogueWindows/DB_Daius` (`BTFunctionLibrary.GetBlackboardValueAsObject` (`self.BB_DialogueUI`))))
  (bind _output_get (set `self.DialogueBoxUI` _asdb_daius))
  (set `/Game/Blueprints/UI_Widgets/NPCDialogueWindows/DB_Daius.DialogueText` (`self.Question`) _output_get)
  (`self.PrepareResponses`))

(event `ResponseReceived`
  (params (ResponseReceived :type Text))
  (`BTFunctionLibrary.SetBlackboardValueAsString` (`self.BB_Response`) (`KismetTextLibrary.Conv_TextToString` ResponseReceived))
  (`Widget.RemoveFromParent` (`self.ResponseOptionsUI`))
  (`self.FinishExecute` true))

(fn `PrepareResponses`
  (bind _returnvalue (`|CreateWidget` "/Game/Blueprints/DialogueTrees/W_ResponseOptionsUI.W_ResponseOptionsUI_C"))
  (bind _output_get (set `self.ResponseOptionsUI` _returnvalue))
  (`Overlay.AddChildToOverlay` (`/Game/Blueprints/UI_Widgets/NPCDialogueWindows/DB_Daius.ResponseOptionsPanel` (`self.DialogueBoxUI`)) _output_get)
  (for _array_element (`self.Responses`)
    (bind _returnvalue_2 (`|CreateWidget` "/Game/Blueprints/DialogueTrees/W_ResponseUI.W_ResponseUI_C" null _array_element))
    (`VerticalBox.AddChildToVerticalBox` (`/Game/Blueprints/DialogueTrees/W_ResponseOptionsUI.ResponseList` (`self.ResponseOptionsUI`)) _returnvalue_2)
    (add `/Game/Blueprints/DialogueTrees/W_ResponseUI.ResponseClicked` _returnvalue_2 (`|CreateDelegate` :!event `ResponseReceived`))))