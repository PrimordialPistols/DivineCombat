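; Behavior tree task that opens the dialogue UI for a BP_DialogueNPC at the start of a conversation.
; It puts the NPC's name into the hub game mode HUD's dialogue box, shows it, and stores that widget in the blackboard.
; It then disables player character input, shows the mouse cursor, and finishes successfully.
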(event `self.ReceiveExecuteAI`
  (params (OwnerController :type "AIController Object Reference") (ControlledPawn :type "Pawn Object Reference"))
  (bind _returnvalue (`GameplayStatics.GetPlayerController` 0))
  (bind _asbp_dialogue_npc (cast `/Game/Blueprints/HubBPs/HubUnits/BP_DialogueNPC` ControlledPawn))
  (set `self.NPCPawn` _asbp_dialogue_npc)
  (bind _asbp_hub_level_game_mode (cast `/Game/Blueprints/GameModes/BP_HubLevelGameMode` (`GameplayStatics.GetGameMode`)))
  (bind _dialoguebox_0 (`/Game/Blueprints/UI_Widgets/NPCDialogueWindows/W_HeadsUpDisplay.DialogueBox_0` (`/Game/Blueprints/GameModes/BP_HubLevelGameMode.HeadsUpDisplay` _asbp_hub_level_game_mode)))
  (set `/Game/Blueprints/UI_Widgets/NPCDialogueWindows/DB_Daius.NameText` (`/Game/Blueprints/HubBPs/HubUnits/BP_DialogueNPC.Name` (`self.NPCPawn`)) _dialoguebox_0)
  (`Widget.SetVisibility` _dialoguebox_0 "Visible")
  (`BTFunctionLibrary.SetBlackboardValueAsObject` (`self.BB_DialogueUI`) _dialoguebox_0)
  (`Actor.DisableInput` (`GameplayStatics.GetPlayerCharacter` 0) _returnvalue)
  (set `PlayerController.bShowMouseCursor` true _returnvalue)
  (`self.FinishExecute` true))