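; Turn-based tactics unit that tracks faction, movement, action and health points on a BP_Grid.
; It snaps to the nearest tile on spawn, captures its icon via render target, and highlights reachable tiles on hover.
; Moves follow a timeline-driven Grid spline, while attacks read DT_Spells to damage or heal tile occupants, updating widgets.
; Turn end refills points; death checks for faction defeat; click handlers are empty, with selection logic unconnected.
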(event `Event_SetReachableIndexes`
  (bind _reachabletiles (`/Game/Blueprints/Grid/BP_Grid.GetReachableIndexes` (`self.grid`) (`self.gridIndex`) (`self.currentMovementPoints`)))
  (set `self.Reachable Indexes` _reachabletiles))

(event `self.ReceiveBeginPlay`
  (bind (_returnvalue_x _returnvalue_y _returnvalue_z) (`KismetMathLibrary.BreakVector` (select `/Game/Blueprints/Controllers/Units/Enum_UnitFactions` (`self.UnitFaction`) :`NewEnumerator0` (`KismetMathLibrary.Conv_LinearColorToVector` (struct :`G` 0.076253 :`B` 0.46875 :`A` 1.0)) :`NewEnumerator1` (`KismetMathLibrary.Conv_LinearColorToVector` (struct :`R` 0.46875 :`G` 0.003366 :`A` 1.0)))))
  (`KismetSystemLibrary.Delay` 0.1)
  (set `self.playerController` (cast `/Game/Blueprints/Controllers/BP_PlayerController` (`GameplayStatics.GetPlayerController` 0) :!pure true))
  (bind _outactors (`GameplayStatics.GetAllActorsOfClass` "/Game/Blueprints/Grid/BP_Grid.BP_Grid_C"))
  (set `self.grid` (`|GetArrayItem` _outactors))
  (`self.SetGridIndexAndSnapToLocation`)
  (bind _output_get (set `self.unitColor` (make `LinearColor` _returnvalue_x _returnvalue_y _returnvalue_z)))
  ;[1 1 1] SetMaterialColor for cones - replaced with real mesh once implemented
  (`MeshComponent.SetVectorParameterValueOnMaterials` (`self.Cone`) "UnitColor" (`KismetMathLibrary.Conv_LinearColorToVector` _output_get))
  (`MeshComponent.SetVectorParameterValueOnMaterials` (`self.Cone1`) "UnitColor" (`KismetMathLibrary.Conv_LinearColorToVector` _output_get))
  (`MeshComponent.SetVectorParameterValueOnMaterials` (`self.Plane`) "UnitColor" (`KismetMathLibrary.Conv_LinearColorToVector` _output_get))
  (`self.Event_CaptureUnitIcon`)
  (bind _output_get_2 (set `self.maxMovementPoints` (`KismetMathLibrary.RandomIntegerInRange` 2 8)))
  (set `self.currentMovementPoints` _output_get_2)
  (bind _output_get_3 (set `self.maxActionPoints` 6))
  (set `self.currentActionPoints` _output_get_3)
  (bind _output_get_4 (set `self.maxHealthPoints` 20))
  (set `self.currentHealthPoints` _output_get_4)
  (set `self.W_MP` (cast `/Game/Blueprints/Grid/W_MovementPoints` (`WidgetComponent.GetWidget` (`/Game/Blueprints/Grid/BP_Grid.W_MP` (`self.grid`))) :!pure true))
  (set `self.W_HP` (cast `/Game/Blueprints/Grid/W_HealthPoints` (`WidgetComponent.GetWidget` (`/Game/Blueprints/Grid/BP_Grid.W_HP` (`self.grid`))) :!pure true))
  (set `self.W_AP` (cast `/Game/Blueprints/Grid/W_ActionPoints` (`WidgetComponent.GetWidget` (`/Game/Blueprints/Grid/BP_Grid.W_AP` (`self.grid`))) :!pure true))
  (set `self.W_Unit` (cast `/Game/Blueprints/Controllers/Units/W_Unit` (`WidgetComponent.GetUserWidgetObject` (`self.Widget`)) :!pure true))
  (`TextBlock.SetText` (`/Game/Blueprints/Controllers/Units/W_Unit.Text_MP` (`self.W_Unit`)) (`KismetTextLibrary.Conv_StringToText` (`KismetStringLibrary.Concat_StrStr` (`KismetStringLibrary.Conv_IntToString` (`self.currentMovementPoints`)) "MP")))
  (`TextBlock.SetText` (`/Game/Blueprints/Controllers/Units/W_Unit.Text_AP` (`self.W_Unit`)) (`KismetTextLibrary.Conv_StringToText` (`KismetStringLibrary.Concat_StrStr` (`KismetStringLibrary.Conv_IntToString` (`self.currentActionPoints`)) "AP")))
  (`ProgressBar.SetPercent` (`/Game/Blueprints/Controllers/Units/W_Unit.PB_HP` (`self.W_Unit`)) (/ (`KismetMathLibrary.Conv_IntToDouble` (`self.currentHealthPoints`)) (`KismetMathLibrary.Conv_IntToDouble` (`self.maxHealthPoints`))))
  ;[1 1 1] Get a reference to the combat UI, to run NextTurn and remove elements as necessary
  (set `self.W_CombatScreen` (`/Game/AI/AI_Blueprints/GameModeTurnSystem_BP.CombatScreen` (cast `/Game/AI/AI_Blueprints/GameModeTurnSystem_BP` (`GameplayStatics.GetGameMode`) :!pure true))))

(event `Event_Selected`
  (`self.Event_SetReachableIndexes`)
  (`self.Event_StartTurn`)
  (`self.SetUnitWidgetVisibility` true))

(event `self.Cone.OnBeginCursorOver`
  (params (TouchedComponent :type "PrimitiveComponent Object Reference"))
  ;[1 1 1] On mouseover of cones (replace with unit model)
  (`self.Event_SetReachableIndexes` :!label _label)
  (`/Game/Blueprints/Grid/BP_Grid.HighlightReachableTiles` (`self.grid`) true (`self.Reachable Indexes`))
  (`self.SetUnitWidgetVisibility` true))

(event `self.Cone1.OnBeginCursorOver`
  (params (TouchedComponent :type "PrimitiveComponent Object Reference"))
  ;[1 1 1] On mouseover of cones (replace with unit model)
  (goto _label))

(event `Event_Deselected`
  (`self.Event_EndTurn`)
  (`self.SetUnitWidgetVisibility` false))

(event `self.Cone.OnEndCursorOver`
  (params (TouchedComponent :type "PrimitiveComponent Object Reference"))
  ;[1 1 1] On mouseover of cones (replace with unit model)
  (`/Game/Blueprints/Grid/BP_Grid.HighlightReachableTiles` (`self.grid`) false (`self.Reachable Indexes`) :!label _label_2)
  (if (!= (`/Game/Blueprints/Controllers/BP_PlayerController.SelectedUnit` (`self.playerController`)) self)
    (`self.SetUnitWidgetVisibility` false)))

(event `self.Cone1.OnEndCursorOver`
  (params (TouchedComponent :type "PrimitiveComponent Object Reference"))
  ;[1 1 1] On mouseover of cones (replace with unit model)
  (goto _label_2))

(event `self.Cone.OnClicked`
  (params (TouchedComponent :type "PrimitiveComponent Object Reference") (ButtonPressed :type "Key Structure"))
  ;[1 1 1] Select unit via click - currently bugged
)

(event `self.Cone1.OnClicked`
  (params (TouchedComponent :type "PrimitiveComponent Object Reference") (ButtonPressed :type "Key Structure"))
  ;[1 1 1] Select unit via click - currently bugged
)

(event `self.CapsuleComponent.OnClicked`
  (params (TouchedComponent :type "PrimitiveComponent Object Reference") (ButtonPressed :type "Key Structure"))
  ;[1 1 1] Select unit via click - currently bugged
)

(event `Event_MoveAlongPath`
  (params (path :type "Array of Vector2D Structure"))
  (bind _path (`self.Path`))
  (bind _w_mp (`self.W_MP`))
  (bind _path_2 (`self.Path`))
  (bind (_returnvalue_x _returnvalue_y _returnvalue_z) (`KismetMathLibrary.BreakVector` (`self.K2_GetActorLocation` self)))
  (bind _spline (`/Game/Blueprints/Grid/BP_Grid.Spline` (`self.grid`)))
  (bind _value (`BlueprintMapLibrary.Map_Find` (`/Game/Blueprints/Grid/BP_Grid.struct_Tiles` (`self.grid`)) (`|GetArrayItem` _path (`KismetArrayLibrary.Array_LastIndex` _path))))
  (set `self.Path` path)
  (`KismetArrayLibrary.Array_Insert` (`self.Path`) (`self.gridIndex`))
  (`self.UnitOnThisTile` (`|GetArrayItem` _path_2 (`KismetArrayLibrary.Array_LastIndex` _path_2)))
  (`SplineComponent.ClearSplinePoints` (`/Game/Blueprints/Grid/BP_Grid.Spline` (`self.grid`)) true)
  (for _array_element (`self.Path`)
    (bind _value_2 (`BlueprintMapLibrary.Map_Find` (`/Game/Blueprints/Grid/BP_Grid.struct_Tiles` (`self.grid`)) _array_element))
    (`SplineComponent.AddSplinePoint` (`/Game/Blueprints/Grid/BP_Grid.Spline` (`self.grid`)) (`KismetMathLibrary.MakeVector` (.x (`.worldLocation_6_A70E36514AE58654E385C8B858E2185E` (break `/Game/Blueprints/Grid/Struct_Tiles` _value_2))) (.y (`.worldLocation_6_A70E36514AE58654E385C8B858E2185E` (break `/Game/Blueprints/Grid/Struct_Tiles` _value_2))) (+ (.z (`.worldLocation_6_A70E36514AE58654E385C8B858E2185E` (break `/Game/Blueprints/Grid/Struct_Tiles` _value_2))) (`CapsuleComponent.CapsuleHalfHeight` (`self.CapsuleComponent`)))) "World" true))
  (set `/Game/Blueprints/Grid/BP_Grid.bIsAUnitMoving` true (`self.grid`))
  (bind _output_get (set `self.currentMovementPoints` (- (`self.currentMovementPoints`) (`.costFromStart_21_80DABD4143A863E2D67A5F8A6FDF5B6E` (break `/Game/Blueprints/Grid/Struct_Tiles` _value)))))
  (`TextBlock.SetText` (`/Game/Blueprints/Controllers/Units/W_Unit.Text_MP` (`self.W_Unit`)) (`KismetTextLibrary.Conv_StringToText` (`KismetStringLibrary.Concat_StrStr` (`KismetStringLibrary.Conv_IntToString` _output_get) "MP")))
  (`TextBlock.SetText` (`/Game/Blueprints/Grid/W_MovementPoints.Text_MP` (`self.W_MP`)) (`KismetTextLibrary.Conv_StringToText` (`KismetStringLibrary.Concat_StrStr` "-" (`KismetStringLibrary.Conv_IntToString` (`.costFromStart_21_80DABD4143A863E2D67A5F8A6FDF5B6E` (break `/Game/Blueprints/Grid/Struct_Tiles` _value))) "MP")))
  (`SceneComponent.K2_SetWorldLocation` (`/Game/Blueprints/Grid/BP_Grid.W_MP` (`self.grid`)) (`KismetMathLibrary.MakeVector` _returnvalue_x _returnvalue_y (+ _returnvalue_z 400.0)) false false)
  (`UserWidget.PlayAnimation` _w_mp (`/Game/Blueprints/Grid/W_MovementPoints.Anim_MP` _w_mp) 0.0 1 "Forward" 1.0 false)
  ;[1 1 1] Animate Unit Moving Along Path
  (`TimelineComponent.SetPlayRate` (`self.MoveAlongPathTimeline`) (/ 1.0 (* (`KismetArrayLibrary.Array_Length` (`self.Path`)) 0.2)))
  (bind (_direction _progression) (`Timeline|MoveAlongPathTimeline` :!via `PlayFromStart`)
    (:`Update`
      (bind _returnvalue (* _progression (`SplineComponent.GetSplineLength` _spline)))
      (`self.K2_SetActorTransform` self (`KismetMathLibrary.MakeTransform` (`SplineComponent.GetLocationAtDistanceAlongSpline` _spline _returnvalue "World") (`SplineComponent.GetRotationAtDistanceAlongSpline` _spline _returnvalue "World")) false false))
    (:`Finished`
      (set `/Game/Blueprints/Grid/BP_Grid.bIsAUnitMoving` false (`self.grid`)))))

(event `Event_StartTurn`
  (`SceneComponent.SetHiddenInGame` (`self.Plane`) false false))

(event `Event_EndTurn`
  (bind _output_get (set `self.currentMovementPoints` (`self.maxMovementPoints`)))
  (`TextBlock.SetText` (`/Game/Blueprints/Controllers/Units/W_Unit.Text_MP` (`self.W_Unit`)) (`KismetTextLibrary.Conv_StringToText` (`KismetStringLibrary.Concat_StrStr` (`KismetStringLibrary.Conv_IntToString` _output_get) "MP")))
  (bind _output_get_2 (set `self.currentActionPoints` (`self.maxActionPoints`)))
  (`TextBlock.SetText` (`/Game/Blueprints/Controllers/Units/W_Unit.Text_AP` (`self.W_Unit`)) (`KismetTextLibrary.Conv_StringToText` (`KismetStringLibrary.Concat_StrStr` (`KismetStringLibrary.Conv_IntToString` _output_get_2) "AP")))
  (`SceneComponent.SetHiddenInGame` (`self.Plane`) true false)
  (`/Game/Blueprints/Grid/BP_Grid.HighlightReachableTiles` (`self.grid`) false (`self.Reachable Indexes`))
  (`self.Event_SetReachableIndexes`))

(event `Event_Attack`
  (params (selectedSpell :type Integer) (index :type "Vector2D Structure"))
  (bind _w_ap (`self.W_AP`))
  (bind (_returnvalue_x _returnvalue_y _returnvalue_z) (`KismetMathLibrary.BreakVector` (`self.K2_GetActorLocation` self)))
  (bind (_value _returnvalue) (`BlueprintMapLibrary.Map_Find` (`/Game/Blueprints/Grid/BP_Grid.struct_Tiles` (`self.grid`)) index))
  (bind _outrownames (`DataTableFunctionLibrary.GetDataTableRowNames` "/Game/Blueprints/Controllers/Units/DT_Spells.DT_Spells"))
  (bind _returnvalue_2 (`|GetDataTableRow` "/Game/Blueprints/Controllers/Units/DT_Spells.DT_Spells" (`|GetArrayItem` _outrownames selectedSpell))
    (:`then`
      (bind (_cost _damage _range _bishealing) (break `/Game/Blueprints/Controllers/Units/Struct_Spells` _returnvalue_2))
      (bind _output_get (set `self.currentActionPoints` (- (`self.currentActionPoints`) _cost)))
      (`TextBlock.SetText` (`/Game/Blueprints/Controllers/Units/W_Unit.Text_AP` (`self.W_Unit`)) (`KismetTextLibrary.Conv_StringToText` (`KismetStringLibrary.Concat_StrStr` (`KismetStringLibrary.Conv_IntToString` _output_get) "AP")))
      (`TextBlock.SetText` (`/Game/Blueprints/Grid/W_ActionPoints.Text_AP` (`self.W_AP`)) (`KismetTextLibrary.Conv_StringToText` (`KismetStringLibrary.Concat_StrStr` "-" (`KismetStringLibrary.Conv_IntToString` _cost) "AP")))
      (`SceneComponent.K2_SetWorldLocation` (`/Game/Blueprints/Grid/BP_Grid.W_AP` (`self.grid`)) (`KismetMathLibrary.MakeVector` _returnvalue_x _returnvalue_y (+ _returnvalue_z 400.0)) false false)
      (`UserWidget.PlayAnimation` _w_ap (`/Game/Blueprints/Grid/W_ActionPoints.Anim_AP` _w_ap) 0.0 1 "Forward" 1.0 false)
      (if (and _returnvalue (!= (`.unitOnTHisTile_29_4F7E2B004ECCFE23E58EE3B2E1E92652` (break `/Game/Blueprints/Grid/Struct_Tiles` _value)) null))
        (`self.Event_Receive Damage` (`.unitOnTHisTile_29_4F7E2B004ECCFE23E58EE3B2E1E92652` (break `/Game/Blueprints/Grid/Struct_Tiles` _value)) _damage _bishealing)))))

(event `Event_Receive Damage`
  (params (damage :type Integer) (isHealing :type Boolean))
  (bind _w_hp (`self.W_HP`))
  (bind _maxhealthpoints (`self.maxHealthPoints`))
  (bind (_returnvalue_x _returnvalue_y _returnvalue_z) (`KismetMathLibrary.BreakVector` (`self.K2_GetActorLocation` self)))
  (if isHealing
    ;[1 1 1] If healing "damage", increase max HP instead of reducing it. If HP would increase above max, set to max
    (bind _output_get (set `self.currentHealthPoints` (+ (`self.currentHealthPoints`) damage)))
    (if (> _output_get _maxhealthpoints)
      (set `self.currentHealthPoints` _maxhealthpoints))
    (`TextBlock.SetText` (`/Game/Blueprints/Grid/W_HealthPoints.Text_HP` (`self.W_HP`)) (`KismetTextLibrary.Conv_StringToText` (`KismetStringLibrary.Concat_StrStr` "+" (`KismetStringLibrary.Conv_IntToString` damage) "HP")))
    (else
      (set `self.currentHealthPoints` (- (`self.currentHealthPoints`) damage))
      (`TextBlock.SetText` (`/Game/Blueprints/Grid/W_HealthPoints.Text_HP` (`self.W_HP`)) (`KismetTextLibrary.Conv_StringToText` (`KismetStringLibrary.Concat_StrStr` "-" (`KismetStringLibrary.Conv_IntToString` damage) "HP")))))
  (`SceneComponent.K2_SetWorldLocation` (`/Game/Blueprints/Grid/BP_Grid.W_HP` (`self.grid`)) (`KismetMathLibrary.MakeVector` _returnvalue_x _returnvalue_y (+ _returnvalue_z 400.0)) false false)
  (`UserWidget.PlayAnimation` _w_hp (`/Game/Blueprints/Grid/W_HealthPoints.Anim_HP` _w_hp) 0.0 1 "Forward" 1.0 false)
  (`ProgressBar.SetPercent` (`/Game/Blueprints/Controllers/Units/W_Unit.PB_HP` (`self.W_Unit`)) (/ (`KismetMathLibrary.Conv_IntToDouble` (`self.currentHealthPoints`)) (`KismetMathLibrary.Conv_IntToDouble` (`self.maxHealthPoints`))))
  (if (<= (`self.currentHealthPoints`) 0)
    (`self.Event_KillUnit` self)))

(event `Event_CaptureUnitIcon`
  (`/Engine/EditorBlueprintResources/StandardMacros.IsValid` (`self.MT_UnitIcon`)
    (:`Is Valid`
      _)
    (:`Is Not Valid`
      (bind _returnvalue (`KismetMaterialLibrary.CreateDynamicMaterialInstance` "/Game/Blueprints/Controllers/Units/MT_UnitIcon.MT_UnitIcon"))
      (set `self.MT_UnitIcon` _returnvalue)))
  (`/Engine/EditorBlueprintResources/StandardMacros.IsValid` (`self.RT_UnitIcon`)
    (:`Is Valid`
      _)
    (:`Is Not Valid`
      (bind _returnvalue_2 (`KismetRenderingLibrary.CreateRenderTarget2D` 256))
      (bind _output_get (set `self.RT_UnitIcon` _returnvalue_2))
      (set `SceneCaptureComponent2D.TextureTarget` _output_get (`self.SceneCaptureComponent2D`))))
  (`SceneCaptureComponent.ShowOnlyActorComponents` (`self.SceneCaptureComponent2D`) self true)
  (`SceneCaptureComponent2D.CaptureScene` (`self.SceneCaptureComponent2D`))
  (`MaterialInstanceDynamic.SetTextureParameterValue` (`self.MT_UnitIcon`) "RenderTargetTexture" (`self.RT_UnitIcon`)))

(event `SetUnitWidgetVisibility`
  (params (visible :type Boolean))
  ;[1 1 1] Sets visibility of unit HP bar and other info - currently visible on unit mouseover or when unit turn is in progress
  (`/Engine/EditorBlueprintResources/StandardMacros.IsValid` (`self.W_Unit`)
    (:`Is Valid`
      (if visible
        (`Widget.SetVisibility` (`self.W_Unit`) "HitTestInvisible")
        (else
          (`Widget.SetVisibility` (`self.W_Unit`) "Hidden"))))))

(event `Event_KillUnit`
  (params (Unit :type "/Game/Blueprints/Controllers/BP_Unit Object Reference"))
  (if (== (`/Game/Blueprints/Controllers/BP_PlayerController.SelectedUnit` (`self.playerController`)) Unit)
    (set `/Game/Blueprints/Controllers/BP_PlayerController.SelectedUnit` null (`self.playerController`)) ; If the entity killed was the selected unit, set selected unit to be null
    (`/Game/Blueprints/Controllers/W_CombatScreen.Event_NextTurn` (`self.W_CombatScreen`)) ; If it was the dying entity's turn, end its turn
  )
  (`self.CheckFactionLossOnDeath` (`/Game/Blueprints/Controllers/BP_Unit.UnitFaction` Unit) Unit))

(fn `CheckFactionLossOnDeath`
  (params (Faction :type "/Game/Blueprints/Controllers/Units/Enum_UnitFactions Enum" :default "NewEnumerator0") (dyingUnit :type "/Game/Blueprints/Controllers/BP_Unit Object Reference"))
  (locals (factionHasLost :type Boolean :default true))
  (bind _w_combatscreen (`self.W_CombatScreen`))
  (bind _outactors (`GameplayStatics.GetAllActorsOfClass` "BP_Unit_C"))
  (for _array_element _outactors
    (if (and (`|EnumEquality` (`/Game/Blueprints/Controllers/BP_Unit.UnitFaction` _array_element) Faction) (!= _array_element dyingUnit))
      (set `local.factionHasLost` false)))
  (`self.K2_DestroyActor` dyingUnit)
  ;[1 1 1] If the faction that has lost is the PlayerFaction, display player loss; Otherwise, display player victory
  (if (`local.factionHasLost`)
    (if (`|EnumEquality` Faction "NewEnumerator0")
      (`/Game/Blueprints/Controllers/W_CombatScreen.Event_DisplayPlayerLoss` _w_combatscreen)
      (else
        (`/Game/Blueprints/Controllers/W_CombatScreen.Event_DisplayPlayerVictory` _w_combatscreen)))))

(fn `SetGridIndexAndSnapToLocation`
  (locals (closestDistance :type "Float (double-precision)") (closestIndex :type "Vector2D Structure"))
  (bind _closestindex (`local.closestIndex`))
  (set `local.closestDistance` 10000000000.0)
  (bind _keys (`BlueprintMapLibrary.Map_Keys` (`/Game/Blueprints/Grid/BP_Grid.struct_Tiles` (`self.grid`))))
  (for _array_element _keys
    (bind _returnvalue (`KismetMathLibrary.VSize` (- (`.worldLocation_6_A70E36514AE58654E385C8B858E2185E` (break `/Game/Blueprints/Grid/Struct_Tiles` (`BlueprintMapLibrary.Map_Find` (`/Game/Blueprints/Grid/BP_Grid.struct_Tiles` (`self.grid`)) _array_element))) (`self.K2_GetActorLocation` self))))
    (if (< _returnvalue (`local.closestDistance`))
      (set `local.closestDistance` _returnvalue)
      (set `local.closestIndex` _array_element)))
  (`self.UnitOnThisTile` _closestindex)
  (set `self.gridIndex` _closestindex)
  (`self.K2_SetActorLocation` (`.worldLocation_6_A70E36514AE58654E385C8B858E2185E` (break `/Game/Blueprints/Grid/Struct_Tiles` (`BlueprintMapLibrary.Map_Find` (`/Game/Blueprints/Grid/BP_Grid.struct_Tiles` (`self.grid`)) (`local.closestIndex`))))))

(fn `UnitOnThisTile`
  (params (gridIndex :type "Vector2D Structure"))
  (bind _struct_tiles (`/Game/Blueprints/Grid/BP_Grid.struct_Tiles` (`self.grid`)))
  (bind _struct_tiles_2 (`/Game/Blueprints/Grid/BP_Grid.struct_Tiles` (`self.grid`)))
  (bind _value (`BlueprintMapLibrary.Map_Find` _struct_tiles (`self.gridIndex`)))
  (bind _value_2 (`BlueprintMapLibrary.Map_Find` _struct_tiles_2 (`self.gridIndex`)))
  (`BlueprintMapLibrary.Map_Add` _struct_tiles_2 (`self.gridIndex`) (make `/Game/Blueprints/Grid/Struct_Tiles` (break `/Game/Blueprints/Grid/Struct_Tiles` _value_2) null (`.groundType_4_5EDF73C242146046D28B8C815B4771E6` (break `/Game/Blueprints/Grid/Struct_Tiles` _value_2)) (`.worldLocation_6_A70E36514AE58654E385C8B858E2185E` (break `/Game/Blueprints/Grid/Struct_Tiles` _value_2)) (`.gridIndex_8_793EB0E84BC077A05BA715917A8EE126` (break `/Game/Blueprints/Grid/Struct_Tiles` _value_2)) (`.tileCost_20_3ECDF8F94CBA04C11D890C906A525AA3` (break `/Game/Blueprints/Grid/Struct_Tiles` _value_2)) (`.finalCOst_11_26A5CBC94BC570F9B422FAB4A2F7B5F2` (break `/Game/Blueprints/Grid/Struct_Tiles` _value_2)) (`.costFromStart_21_80DABD4143A863E2D67A5F8A6FDF5B6E` (break `/Game/Blueprints/Grid/Struct_Tiles` _value_2)) (`.estimatedCostToTarget_22_AE78572B4FF86D0C8E95BA886348A4A9` (break `/Game/Blueprints/Grid/Struct_Tiles` _value_2)) (`.previousTile_26_8E277672415381B91A0E929898E2BEBF` (break `/Game/Blueprints/Grid/Struct_Tiles` _value_2))))
  (set `self.gridIndex` gridIndex)
  (`BlueprintMapLibrary.Map_Add` _struct_tiles (`self.gridIndex`) (make `/Game/Blueprints/Grid/Struct_Tiles` (break `/Game/Blueprints/Grid/Struct_Tiles` _value) self (`.groundType_4_5EDF73C242146046D28B8C815B4771E6` (break `/Game/Blueprints/Grid/Struct_Tiles` _value)) (`.worldLocation_6_A70E36514AE58654E385C8B858E2185E` (break `/Game/Blueprints/Grid/Struct_Tiles` _value)) (`.gridIndex_8_793EB0E84BC077A05BA715917A8EE126` (break `/Game/Blueprints/Grid/Struct_Tiles` _value)) (`.tileCost_20_3ECDF8F94CBA04C11D890C906A525AA3` (break `/Game/Blueprints/Grid/Struct_Tiles` _value)) (`.finalCOst_11_26A5CBC94BC570F9B422FAB4A2F7B5F2` (break `/Game/Blueprints/Grid/Struct_Tiles` _value)) (`.costFromStart_21_80DABD4143A863E2D67A5F8A6FDF5B6E` (break `/Game/Blueprints/Grid/Struct_Tiles` _value)) (`.estimatedCostToTarget_22_AE78572B4FF86D0C8E95BA886348A4A9` (break `/Game/Blueprints/Grid/Struct_Tiles` _value)) (`.previousTile_26_8E277672415381B91A0E929898E2BEBF` (break `/Game/Blueprints/Grid/Struct_Tiles` _value)))))

(fn `UserConstructionScript`)