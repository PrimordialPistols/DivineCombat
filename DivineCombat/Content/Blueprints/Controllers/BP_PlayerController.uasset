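; Player controller for a grid-based tactics game, handling unit selection, path movement, spell targeting and camera zoom.
; Number keys or right-click (the unit's weapon from DT_UnitStatistics) toggle a spell.
; DT_Spells supplies cost and range pattern, which the Grid paints if action points suffice; validated targets trigger the unit's attack.
; Zoom eases spring arm length and ortho width together; debug keys cover obstacle visibility, slow motion and goal tracking.
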(event `self.ReceiveBeginPlay`
  ;[1 1 1] Set Local Reference to Actor Pawn
  (set `self.aPawn` (cast `/Game/Blueprints/Controllers/BP_Pawn` (`self.K2_GetPawn`) :!pure true))
  (`KismetSystemLibrary.Delay` 0.2)
  ;[1 1 1] Hide Unit Widgets by Default
  (bind _outactors (`GameplayStatics.GetAllActorsOfClass` "/Game/Blueprints/GridBPs/GridUnits/BP_Unit.BP_Unit_C"))
  (for _array_element _outactors
    (`/Game/Blueprints/GridBPs/GridUnits/BP_Unit.SetUnitWidgetVisibility` _array_element false)))

(event `InputAxis|Zoom`
  (params (AxisValue :type "Float (single-precision)"))
  ;[1 1 1] Fire Zoom event on Mousewheel scroll
  (`self.Zoom` AxisValue))

(event `Event_NewUnitSelected`
  (params (unit :type "/Game/Blueprints/GridBPs/GridUnits/BP_Unit Object Reference"))
  ;[1 1 1] Ensure new selected unit is valid, and deselect all spells upon new unit selection
  (`/Engine/EditorBlueprintResources/StandardMacros.IsValid` (`self.SelectedUnit`)
    (:`Is Valid`
      (`/Game/Blueprints/GridBPs/GridUnits/BP_Unit.Event_Deselected` (`self.SelectedUnit`)))
    (:`Is Not Valid`
      _))
  (bind _output_get (set `self.SelectedUnit` unit))
  (`/Engine/EditorBlueprintResources/StandardMacros.IsValid` _output_get
    (:`Is Valid`
      (`/Game/Blueprints/GridBPs/GridUnits/BP_Unit.Event_Selected` _output_get)
      (`self.Event_DeselectAllSpells`))))

(event `Event_NewPathAvailable`
  (params (path :type "Array of Vector2D Structure"))
  ;[1 1 1] Fire Event_MoveAlongPath if SelectedUnit is valid, and no spell is selected
  (if (== (`self.spellSelected`) -1)
    (`/Engine/EditorBlueprintResources/StandardMacros.IsValid` (`self.SelectedUnit`)
      (:`Is Valid`
        (`/Game/Blueprints/GridBPs/GridUnits/BP_Unit.Event_MoveAlongPath` (`self.SelectedUnit`) path)))))

(event `Key|R`
  (params (Key :type "Key Structure"))
  ;[1 1 1] Debug World Manipulation Code - Hide Obstacles, Changed Game Speed
  (:`Pressed`
    (`/Engine/EditorBlueprintResources/StandardMacros.FlipFlop`
      (:`A`
        (bind _outactors (`GameplayStatics.GetAllActorsOfClass` "/Game/Blueprints/GridBPs/GridObjects/BP_BaseObstacle.BP_BaseObstacle_C"))
        (for _array_element _outactors
          (`self.SetActorHiddenInGame` _array_element false)))
      (:`B`
        (bind _outactors_2 (`GameplayStatics.GetAllActorsOfClass` "/Game/Blueprints/GridBPs/GridObjects/BP_BaseObstacle.BP_BaseObstacle_C"))
        (for _array_element_2 _outactors_2
          (`self.SetActorHiddenInGame` _array_element_2 false))))))

(event `Key|T`
  (params (Key :type "Key Structure"))
  ;[1 1 1] Debug World Manipulation Code - Hide Obstacles, Changed Game Speed
  (:`Pressed`
    (`/Engine/EditorBlueprintResources/StandardMacros.FlipFlop`
      (:`A`
        (`GameplayStatics.SetGlobalTimeDilation` 0.1))
      (:`B`
        (`GameplayStatics.SetGlobalTimeDilation` 1.0)))))

(event `Key|One`
  (params (Key :type "Key Structure"))
  ;[1 1 1] Stopgap Spell Selection - Set currently selected spell for the player, fire SpellSelected Event
  (:`Pressed`
    (set `self.spellSelected` (`KismetMathLibrary.SelectInt` -1 0 (== (`self.spellSelected`) 0)))
    (`self.Event_SpellSelected` :!label _label)))

(event `Key|Two`
  (params (Key :type "Key Structure"))
  ;[1 1 1] Stopgap Spell Selection - Set currently selected spell for the player, fire SpellSelected Event
  (:`Pressed`
    (set `self.spellSelected` (`KismetMathLibrary.SelectInt` -1 1 (== (`self.spellSelected`) 1)))
    (goto _label)))

(event `Key|Three`
  (params (Key :type "Key Structure"))
  ;[1 1 1] Stopgap Spell Selection - Set currently selected spell for the player, fire SpellSelected Event
  (:`Pressed`
    (set `self.spellSelected` (`KismetMathLibrary.SelectInt` -1 2 (== (`self.spellSelected`) 2)))
    (goto _label)))

(event `Key|Four`
  (params (Key :type "Key Structure"))
  ;[1 1 1] Stopgap Spell Selection - Set currently selected spell for the player, fire SpellSelected Event
  (:`Pressed`
    (set `self.spellSelected` (`KismetMathLibrary.SelectInt` -1 3 (== (`self.spellSelected`) 3)))
    (goto _label)))

(event `Key|RightMouseButton`
  (params (Key :type "Key Structure"))
  (:`Pressed`
    (bind _outrownames (`DataTableFunctionLibrary.GetDataTableRowNames` "/Game/DataStructures/DT_UnitStatistics.DT_UnitStatistics"))
    (bind _returnvalue (`|GetDataTableRow` "/Game/DataStructures/DT_UnitStatistics.DT_UnitStatistics" (`|GetArrayItem` _outrownames (- (`/Game/Blueprints/GridBPs/GridUnits/BP_Unit.UnitType` (`self.SelectedUnit`)) 1)))
      (:`then`
        (bind _spell_index (`self.DetermineWeaponFromUnitType` (`.WeaponType_35_4FC064B64CA15DC96F39E3BF711B957A` (break `/Game/DataStructures/Struct_UnitStats` _returnvalue))))
        (set `self.spellSelected` (`KismetMathLibrary.SelectInt` -1 _spell_index (== (`self.spellSelected`) _spell_index)))
        (`self.Event_SpellSelected`)))))

(event `Event_SpellSelected`
  (bind _selectedunit (`self.SelectedUnit`))
  (bind _grid (`self.grid`))
  ;[1 1 1] Search Data Table of Spells for the selected index
  (if (!= (`self.spellSelected`) -1)
    (bind _outrownames (`DataTableFunctionLibrary.GetDataTableRowNames` "/Game/DataStructures/DT_Spells.DT_Spells"))
    (bind _returnvalue (`|GetDataTableRow` "/Game/DataStructures/DT_Spells.DT_Spells" (`|GetArrayItem` _outrownames (`self.spellSelected`)))
      (:`then`
        (bind (_cost _damage _range _bishealing _cooldown _aoerange _criticalchance _criticaldamage _bcanattackthroughwalls _pattern _patternrangemin _patternrangemax) (break `/Game/DataStructures/Struct_Spells` _returnvalue))
        ;[1 1 1] Based on Selected Spell, create targetting pattern to be painted on grid based on spell type, and maximum and minimum spell range
        (if (>= (`/Game/Blueprints/GridBPs/GridUnits/BP_Unit.currentActionPoints` _selectedunit) _cost)
          (switch `/Game/DataStructures/Enum_Patterns` _pattern
            (:`NewEnumerator5`
              (`/Game/Blueprints/GridBPs/GridObjects/BP_Grid.Event_NewSpellSelected` (`self.grid`) (`/Game/Blueprints/GridBPs/GridUnits/BP_Unit.gridIndex` _selectedunit) _range))
            (:`NewEnumerator0`
              (`/Game/Blueprints/GridBPs/GridObjects/BP_Grid.Event_NewSpellSelected` (`self.grid`) (`/Game/Blueprints/GridBPs/GridUnits/BP_Unit.gridIndex` _selectedunit) (`/Game/Blueprints/GridBPs/GridObjects/BP_Grid.GetLinearPattern` _grid _patternrangemin _patternrangemax)))
            (:`NewEnumerator1`
              (`/Game/Blueprints/GridBPs/GridObjects/BP_Grid.Event_NewSpellSelected` (`self.grid`) (`/Game/Blueprints/GridBPs/GridUnits/BP_Unit.gridIndex` _selectedunit) (`/Game/Blueprints/GridBPs/GridObjects/BP_Grid.GetDiagonalPattern` _grid _patternrangemin _patternrangemax)))
            (:`NewEnumerator2`
              (`/Game/Blueprints/GridBPs/GridObjects/BP_Grid.Event_NewSpellSelected` (`self.grid`) (`/Game/Blueprints/GridBPs/GridUnits/BP_Unit.gridIndex` _selectedunit) (`/Game/Blueprints/GridBPs/GridObjects/BP_Grid.GetDiamondPattern` _grid _patternrangemin _patternrangemax)))
            (:`NewEnumerator3`
              (`/Game/Blueprints/GridBPs/GridObjects/BP_Grid.Event_NewSpellSelected` (`self.grid`) (`/Game/Blueprints/GridBPs/GridUnits/BP_Unit.gridIndex` _selectedunit) (`/Game/Blueprints/GridBPs/GridObjects/BP_Grid.GetSquarePattern` _grid _patternrangemin _patternrangemax))))
          (else
            (`self.Event_DeselectAllSpells`))))
      (:`RowNotFound`
        (`self.Event_DeselectAllSpells`)))
    (else
      (`self.Event_DeselectAllSpells`))))

(event `Event_DeselectAllSpells`
  (`/Game/Blueprints/GridBPs/GridObjects/BP_Grid.Event_NewSpellSelected` (`self.grid`) (-1.0 -1.0) (`|MakeArray` (0.0 0.0) :!type "Vector2D Structure"))
  (set `self.spellSelected` -1))

(event `Event_SpellValidated`
  (params (index :type "Vector2D Structure"))
  (`/Game/Blueprints/GridBPs/GridUnits/BP_Unit.Event_Attack` (`self.SelectedUnit`) (`self.spellSelected`) index)
  (`self.Event_DeselectAllSpells`))

(event `Event_SpellCancelled`
  (`self.Event_DeselectAllSpells`))

(event `Key|Q`
  (params (Key :type "Key Structure"))
  (bind _grid (`self.grid`))
  (:`Pressed`
    (`/Game/Blueprints/GridBPs/GridObjects/BP_Grid.IncrementGoalTrackerByName` _grid (`/Game/Blueprints/GridBPs/GridObjects/BP_Grid.GoalTrackersStructs` _grid) "Q-Presser")))

(fn `DetermineWeaponFromUnitType`
  (params (`Weapon Type` :type "/Game/DataStructures/Enum_WeaponType Enum" :default "NewEnumerator0"))
  (returns (`Spell Index` :type Integer))
  (locals (LocalIndex :type Integer))
  (switch `/Game/DataStructures/Enum_WeaponType` `Weapon Type`
    (:`NewEnumerator0`
      (set `local.LocalIndex` 0))
    (:`NewEnumerator1`
      (set `local.LocalIndex` 1))
    (:`NewEnumerator2`
      (set `local.LocalIndex` 2))
    (:`NewEnumerator3`
      (set `local.LocalIndex` 3))
    (:`NewEnumerator5`
      (set `local.LocalIndex` 5)))
  (return (`local.LocalIndex`)))

(fn `UserConstructionScript`)

(fn `Zoom`
  (params (zoomAmount :type "Float (double-precision)"))
  (bind _returnvalue (<= (`self.cameraDesiredZoomLevel`) (`self.cameraZoomMax`)))
  ;[1 1 1] Determine Desired Zoom Level Based on Mouse Scroll, Clamping at Max and Min Values
  (set `self.cameraDesiredZoomLevel` (+ (`self.cameraDesiredZoomLevel`) (* (- 0.0 zoomAmount) (`self.cameraZoomSpeed`))))
  (bind _output_get (set `self.cameraDesiredZoomLevel` (`KismetMathLibrary.SelectFloat` (`self.cameraDesiredZoomLevel`) (`KismetMathLibrary.SelectFloat` (`KismetMathLibrary.Lerp` (`self.cameraDesiredZoomLevel`) (`self.cameraZoomMin`) 0.2) (`KismetMathLibrary.Lerp` (`self.cameraDesiredZoomLevel`) (`self.cameraZoomMax`) 0.2) _returnvalue) (and (>= (`self.cameraDesiredZoomLevel`) (`self.cameraZoomMin`)) _returnvalue))))
  (bind _returnvalue_2 (`KismetMathLibrary.Lerp` (`SpringArmComponent.TargetArmLength` (`/Game/Blueprints/Controllers/BP_Pawn.SpringArm` (`self.aPawn`))) _output_get 0.1))
  ;[1 1 1] Once Desired Zoom Level is set, adjust camera arm length & adjust camera ortho to pan in/out
  (set `SpringArmComponent.TargetArmLength` _returnvalue_2 (`/Game/Blueprints/Controllers/BP_Pawn.SpringArm` (`self.aPawn`)))
  (`CameraComponent.SetOrthoWidth` (`/Game/Blueprints/Controllers/BP_Pawn.Camera` (`self.aPawn`)) (* _returnvalue_2 1.2)))