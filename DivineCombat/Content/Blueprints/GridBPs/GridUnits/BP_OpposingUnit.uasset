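; Opposing grid unit Blueprint for weapon-triangle combat against a DefaultUnit, with its own health, damage and weapon flags.
; HealthDecrease destroys the actor once Unit2Health reaches zero or below; a duplicate check in EventGraph is disconnected.
; Unit2WeaponTriangle holds unwired draft logic: sword beats axe, axe beats spear, spear beats sword, with wins raising this unit's damage and lowering DefaultUnit's.
; BeginPlay, Tick and the construction script are empty.
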(event `self.ReceiveBeginPlay`)

(event `self.ReceiveTick`
  (params (DeltaSeconds :type "Float (single-precision)")))

(fn `Health Decrease`
  (if (<= (`self.Unit2_Health`) 0)
    (`self.K2_DestroyActor`)))

(fn `Unit2_WeaponTriangle`)

(fn `UserConstructionScript`)