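; Battle dialogue manager that plays pre-battle and post-battle dialogue through its AI_DialogueNPC controller.
; LoadMapDialogue picks intro and win behavior trees from the level name and player Divine, treating any level other than Forest or Castle as Colosseum.
; The pre-battle event hands the intro tree to the controller before starting it.
; The post-battle event only calls StartDialogue2, without passing the stored win tree.
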(event `self.ReceiveBeginPlay`)

(event `PlayPrebattleDialogue`
  (bind _asai_dialogue_npc (cast `/Game/Blueprints/HubBPs/HubUnits/AI_DialogueNPC` (`AIBlueprintHelperLibrary.GetAIController` self)))
  (set `/Game/Blueprints/HubBPs/HubUnits/AI_DialogueNPC.DialogueTree` (`self.DialogueTree`) _asai_dialogue_npc)
  (`/Game/Blueprints/HubBPs/HubUnits/AI_DialogueNPC.StartDialogue` _asai_dialogue_npc))

(event `PlayPostbattleDialogue`
  (bind _asai_dialogue_npc (cast `/Game/Blueprints/HubBPs/HubUnits/AI_DialogueNPC` (`AIBlueprintHelperLibrary.GetAIController` self)))
  (`/Game/Blueprints/HubBPs/HubUnits/AI_DialogueNPC.StartDialogue2` _asai_dialogue_npc))

(fn `LoadMapDialogue`
  (params (`Player Divine` :type "/Game/DataStructures/Enum_Divine Enum" :default "NewEnumerator0"))
  (bind _returnvalue (`GameplayStatics.GetCurrentLevelName` true))
  (if (`KismetStringLibrary.EqualEqual_StrStr` _returnvalue "M_ForestBattle")
    (switch `/Game/DataStructures/Enum_Divine` `Player Divine` ; Forest
      (:`NewEnumerator0`
        (set `self.DialogueTree` "/Game/Blueprints/DialogueTrees/FinishedTrees/Forest/BT_ForestMelIntro.BT_ForestMelIntro")
        (set `self.DialogueTree2` "/Game/Blueprints/DialogueTrees/FinishedTrees/Forest/BT_ForestMelWin.BT_ForestMelWin"))
      (:`NewEnumerator1`
        (set `self.DialogueTree` "/Game/Blueprints/DialogueTrees/FinishedTrees/Forest/BT_ForestAeliaIntro.BT_ForestAeliaIntro")
        (set `self.DialogueTree2` "/Game/Blueprints/DialogueTrees/FinishedTrees/Forest/BT_ForestAeliaWin.BT_ForestAeliaWin"))
      (:`NewEnumerator2`
        (set `self.DialogueTree` "/Game/Blueprints/DialogueTrees/FinishedTrees/Forest/BT_ForestAevumIntro.BT_ForestAevumIntro")
        (set `self.DialogueTree2` "/Game/Blueprints/DialogueTrees/FinishedTrees/Forest/BT_ForestAevumWin.BT_ForestAevumWin"))
      (:`NewEnumerator3`
        (set `self.DialogueTree` "/Game/Blueprints/DialogueTrees/FinishedTrees/Forest/BT_ForestHeroIntro.BT_ForestHeroIntro")
        (set `self.DialogueTree2` "/Game/Blueprints/DialogueTrees/FinishedTrees/Forest/BT_ForestHeroWin.BT_ForestHeroWin")))
    (elif (`KismetStringLibrary.EqualEqual_StrStr` _returnvalue "M_CastleBattle")
      (switch `/Game/DataStructures/Enum_Divine` `Player Divine` ; Castle
        (:`NewEnumerator0`
          (set `self.DialogueTree` "/Game/Blueprints/DialogueTrees/FinishedTrees/Castle/BT_CastleMelIntro.BT_CastleMelIntro")
          (set `self.DialogueTree2` "/Game/Blueprints/DialogueTrees/FinishedTrees/Castle/BT_CastleMelWin.BT_CastleMelWin"))
        (:`NewEnumerator1`
          (set `self.DialogueTree` "/Game/Blueprints/DialogueTrees/FinishedTrees/Castle/BT_CastleAeliaIntro.BT_CastleAeliaIntro")
          (set `self.DialogueTree2` "/Game/Blueprints/DialogueTrees/FinishedTrees/Castle/BT_CastleAeliaWin.BT_CastleAeliaWin"))
        (:`NewEnumerator2`
          (set `self.DialogueTree` "/Game/Blueprints/DialogueTrees/FinishedTrees/Castle/BT_CastleAevumIntro.BT_CastleAevumIntro")
          (set `self.DialogueTree2` "/Game/Blueprints/DialogueTrees/FinishedTrees/Castle/BT_CastleAevumWin.BT_CastleAevumWin"))
        (:`NewEnumerator3`
          (set `self.DialogueTree` "/Game/Blueprints/DialogueTrees/FinishedTrees/Castle/BT_CastleHeroIntro.BT_CastleHeroIntro")
          (set `self.DialogueTree2` "/Game/Blueprints/DialogueTrees/FinishedTrees/Castle/BT_CastleHeroWin.BT_CastleHeroWin")))
      (else
        (switch `/Game/DataStructures/Enum_Divine` `Player Divine` ; Colosseum
          (:`NewEnumerator0`
            (set `self.DialogueTree` "/Game/Blueprints/DialogueTrees/FinishedTrees/Colosseum/BT_ColoMelIntro.BT_ColoMelIntro")
            (set `self.DialogueTree2` "/Game/Blueprints/DialogueTrees/FinishedTrees/Colosseum/BT_ColoMelWin.BT_ColoMelWin"))
          (:`NewEnumerator1`
            (set `self.DialogueTree` "/Game/Blueprints/DialogueTrees/FinishedTrees/Colosseum/BT_ColoAeliaIntro.BT_ColoAeliaIntro")
            (set `self.DialogueTree2` "/Game/Blueprints/DialogueTrees/FinishedTrees/Colosseum/BT_ColoAeliaWin.BT_ColoAeliaWin"))
          (:`NewEnumerator2`
            (set `self.DialogueTree` "/Game/Blueprints/DialogueTrees/FinishedTrees/Colosseum/BT_ColoAevumIntro.BT_ColoAevumIntro")
            (set `self.DialogueTree2` "/Game/Blueprints/DialogueTrees/FinishedTrees/Colosseum/BT_ColoAevumWin.BT_ColoAevumWin"))
          (:`NewEnumerator3`
            (set `self.DialogueTree` "/Game/Blueprints/DialogueTrees/FinishedTrees/Colosseum/BT_ColoHeroIntro.BT_ColoHeroIntro")
            (set `self.DialogueTree2` "/Game/Blueprints/DialogueTrees/FinishedTrees/Colosseum/BT_ColoHeroWin.BT_ColoHeroWin")))))))

(fn `UserConstructionScript`)