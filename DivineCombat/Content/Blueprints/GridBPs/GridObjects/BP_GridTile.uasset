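; Clickable tile actor for a tactics grid that shows terrain and state, reports hover and selection to the Grid, and scales to its tile size.
; Clicks spawn the PlayerController's chosen unit on empty spawn-zone tiles, or validate or cancel selected spells elsewhere.
; State events set flags and rerun SetTileColor, a priority-ordered sequence where later states override ground-type color through material parameters.
; Tactics mode reveals tiles and their info widget.
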(event `self.ReceiveBeginPlay`
  ;[1 1 1] Initialize Values on Startup - Size, Color, Displayed Numbers
  (`KismetSystemLibrary.Delay` 0.2)
  (`self.SetTileColor`)
  (`self.SetTileSize`)
  (`self.SetWidgetVariables`)
  (`self.Event_ToggleTacticsMode` false))

(event `self.StaticMesh.OnBeginCursorOver`
  (params (TouchedComponent :type "PrimitiveComponent Object Reference"))
  ;[1 1 1] Fire NewTileHovered Grid Event on mouseover
  (`self.Event_StartHoverTile`)
  (`/Game/Blueprints/GridBPs/GridObjects/BP_Grid.Event_NewTileHovered` (`self.Grid`) self))

(event `self.StaticMesh.OnEndCursorOver`
  (params (TouchedComponent :type "PrimitiveComponent Object Reference"))
  ;[1 1 1] Fire NewTileHovered Grid Event on mouseover
  (`/Game/Blueprints/GridBPs/GridObjects/BP_Grid.Event_NewTileHovered` (`self.Grid`) null))

(event `Event_ToggleTacticsMode`
  (params (bIsTactics :type Boolean))
  ;[1 1 1] Display Tile Info Via Color and Widget upon Enabling Tactics Mode
  (set `self.bIsTactics` bIsTactics)
  (`SceneComponent.SetHiddenInGame` (`self.Widget`) (not (`self.bIsTactics`)) false)
  (`self.SetTileColor`))

(event `self.StaticMesh.OnClicked`
  (params (TouchedComponent :type "PrimitiveComponent Object Reference") (ButtonPressed :type "Key Structure"))
  (bind _playercontroller (`self.playerController`))
  (bind _playercontroller_2 (`self.playerController`))
  (bind _currentselector (`/Game/Blueprints/Controllers/BP_PlayerController.CurrentSelector` _playercontroller_2))
  (bind _unittospawn (`/Game/Blueprints/Controllers/BP_PlayerController.UnitToSpawn` _playercontroller_2))
  (bind _value (`BlueprintMapLibrary.Map_Find` (`/Game/Blueprints/GridBPs/GridObjects/BP_Grid.struct_Tiles` (`self.Grid`)) (`self.GridIndex`)))
  ;[1 1 1] Fire Grid events upon clicking on grid
  (`self.Event_SelectTile`)
  (`/Game/Blueprints/GridBPs/GridObjects/BP_Grid.Event_NewTileSelected` (`self.Grid`) self)
  (if (not (`self.bIsSpawnZone`))
    (if (!= (`/Game/Blueprints/Controllers/BP_PlayerController.spellSelected` (`self.playerController`)) -1)
      (if (`self.bIsTargetted`)
        (`/Game/Blueprints/Controllers/BP_PlayerController.Event_SpellValidated` _playercontroller (`self.GridIndex`))
        (else
          (`/Game/Blueprints/Controllers/BP_PlayerController.Event_SpellCancelled` _playercontroller))))
    (elif (== (`.unitOnTHisTile_29_4F7E2B004ECCFE23E58EE3B2E1E92652` (break `/Game/DataStructures/Struct_Tiles` _value)) null)
      (`KismetSystemLibrary.PrintString` "Trying to spawn")
      (if (!= _unittospawn null)
        (bind _returnvalue (`|SpawnActorFromClass` _unittospawn (`KismetMathLibrary.Conv_VectorToTransform` (`.worldLocation_6_A70E36514AE58654E385C8B858E2185E` (break `/Game/DataStructures/Struct_Tiles` _value))) "AdjustIfPossibleButAlwaysSpawn" "OverrideRootScale" null null))
        (`/Game/Blueprints/GridBPs/GridUnits/BP_Unit.SetGridIndexAndSnapToLocation` _returnvalue)
        (set `/Game/Blueprints/Controllers/BP_PlayerController.UnitToSpawn` _unittospawn _playercontroller_2)
        (`/Game/Blueprints/UI_Widgets/Combat/W_UnitSelector.DisableSelector` _currentselector)
        (bind _output_get (set `/Game/Blueprints/GridBPs/GridUnits/BP_Unit.Selector` _currentselector _returnvalue))
        (set `/Game/Blueprints/Controllers/BP_PlayerController.CurrentSelector` _output_get _playercontroller_2)))))

(event `Event_SelectTile`
  ;[1 1 1] Tile Color Change Events
  (set `self.IsSelected` true)
  (`self.SetTileColor` :!label _label))

(event `Event_DeselectTile`
  ;[1 1 1] Tile Color Change Events
  (set `self.IsSelected` false)
  (goto _label))

(event `Event_IsInPath`
  (params (bIsInPath :type Boolean))
  ;[1 1 1] Tile Color Change Events
  (set `self.bIsInPath` bIsInPath)
  (`self.SetTileColor`))

(event `Event_IsReachableByPlayer`
  (params (bIsInPath :type Boolean))
  ;[1 1 1] Tile Color Change Events
  (set `self.bIsReachableByPlayer` bIsInPath)
  (`self.SetTileColor`))

(event `Event_IsReachableByEnemy`
  (params (bIsInPath :type Boolean))
  ;[1 1 1] Tile Color Change Events
  (set `self.bIsReachableByEnemy` bIsInPath)
  (`self.SetTileColor`))

(event `Event_StartHoverTile`
  ;[1 1 1] Tile Color Change Events
  (set `self.IsHovered` true)
  (`self.SetTileColor` :!label _label_2))

(event `Event_EndHoverTile`
  ;[1 1 1] Tile Color Change Events
  (set `self.IsHovered` false)
  (goto _label_2))

(event `Event_TargetTile`
  ;[1 1 1] Tile Color Change Events
  (set `self.bIsTargetted` true)
  (`self.SetTileColor` :!label _label_3))

(event `Event_CancelTargetTile`
  ;[1 1 1] Tile Color Change Events
  (set `self.bIsTargetted` false)
  (goto _label_3))

(event `Event_SetSpawnZone`
  ;[1 1 1] Tile Color Change Events
  (set `self.bIsSpawnZone` true)
  (`self.SetTileColor`))

(event `Event_DisableSpawnZone`
  ;[1 1 1] Tile Color Change Events
  (set `self.bIsSpawnZone` false)
  (`self.SetTileColor`))

(event `Event_SetDamageTiles`
  ;[1 1 1] Pass in the PassThroughDamage and StoodOnDamage values. Then, set the amount of damage that the unit will take
  (set `self.PassThroughDamage` (`/Game/Blueprints/GridBPs/GridObjects/BP_Grid.PassThroughDamage` (`self.Grid`)))
  (set `self.StoodOnDamage` (`/Game/Blueprints/GridBPs/GridObjects/BP_Grid.StoodOnDamage` (`self.Grid`)))
  (set `self.DamageAmount` 10)
  (`self.SetTileColor`))

(event `DebugEvent_OpenSet`
  ;[1 1 1] Not in Use - Debug Pathfinding Visualization
  (`MeshComponent.SetVectorParameterValueOnMaterials` (`self.StaticMesh`) "TileColor" (`KismetMathLibrary.Conv_LinearColorToVector` (struct :`G` 0.46875 :`B` 0.275816 :`A` 1.0))))

(event `DebugEvent_ClosedSet`
  ;[1 1 1] Not in Use - Debug Pathfinding Visualization
  (`MeshComponent.SetVectorParameterValueOnMaterials` (`self.StaticMesh`) "TileColor" (`KismetMathLibrary.Conv_LinearColorToVector` (struct :`R` 0.666667 :`G` 0.092286 :`A` 1.0))))

(fn `GetTileData`
  (returns (Value :type "/Game/DataStructures/Struct_Tiles Structure"))
  (return (`BlueprintMapLibrary.Map_Find` (`/Game/Blueprints/GridBPs/GridObjects/BP_Grid.struct_Tiles` (`self.Grid`)) (`self.GridIndex`))))

(fn `SetTileColor`
  (locals (tileColor :type "LinearColor Structure"))
  (bind (_value_tileactor _value_unitonthistile _value_groundtype) (break `/Game/DataStructures/Struct_Tiles` (`self.GetTileData`)))
  (`|ExecutionSequence`
    (:`then_0`
      (if (`self.bIsTactics`)
        (`MeshComponent.SetScalarParameterValueOnMaterials` (`self.StaticMesh`) "bIsVisible" 1.0)
        (else
          (`MeshComponent.SetScalarParameterValueOnMaterials` (`self.StaticMesh`) "bIsVisible" 0.0))))
    (:`then_1`
      (switch `/Game/DataStructures/Enum_GroundTypes` _value_groundtype
        (:`NewEnumerator0`
          (set `local.tileColor` (struct :`R` 0.713542 :`G` 0.713542 :`B` 0.713542 :`A` 1.0)))
        (:`NewEnumerator1`
          (set `local.tileColor` (struct :`R` 1.0 :`G` 0.917865 :`B` 0.247905 :`A` 1.0)))
        (:`NewEnumerator2`
          (set `local.tileColor` (struct :`R` 1.0 :`G` 0.359765 :`B` 0.148505 :`A` 1.0)))
        (:`NewEnumerator3`
          (set `local.tileColor` (struct :`R` 0.322917 :`B` 0.017967 :`A` 1.0)))
        (:`NewEnumerator4`
          (set `local.tileColor` (struct :`R` 0.026042 :`G` 0.026042 :`B` 0.026042 :`A` 1.0)))))
    (:`then_2`
      (if (`self.IsSelected`)
        (`MeshComponent.SetScalarParameterValueOnMaterials` (`self.StaticMesh`) "IsSelected" 1.0)
        (`MeshComponent.SetScalarParameterValueOnMaterials` (`self.StaticMesh`) "bIsVisible" 1.0)
        (else
          (`MeshComponent.SetScalarParameterValueOnMaterials` (`self.StaticMesh`) "IsSelected" 0.0))))
    (:`then_3`
      (if (`self.bIsReachableByPlayer`)
        (set `local.tileColor` (struct :`R` 0.156006 :`G` 0.214704 :`B` 0.421875 :`A` 1.0))
        (`MeshComponent.SetScalarParameterValueOnMaterials` (`self.StaticMesh`) "bIsVisible" 1.0)))
    (:`then_4`
      (if (`self.bIsReachableByEnemy`)
        (set `local.tileColor` (struct :`R` 0.421875 :`G` 0.156006 :`B` 0.160437 :`A` 1.0))
        (`MeshComponent.SetScalarParameterValueOnMaterials` (`self.StaticMesh`) "bIsVisible" 1.0)))
    (:`then_5`
      (if (`self.bIsInPath`)
        (set `local.tileColor` (struct :`G` 0.071293 :`B` 0.322917 :`A` 1.0))
        (`MeshComponent.SetScalarParameterValueOnMaterials` (`self.StaticMesh`) "bIsVisible" 1.0)))
    (:`then_6`
      (if (`self.bIsTargetted`)
        (set `local.tileColor` (struct :`R` 0.796875 :`G` 0.16555 :`A` 1.0))
        (`MeshComponent.SetScalarParameterValueOnMaterials` (`self.StaticMesh`) "bIsVisible" 1.0)))
    (:`then_7`
      (if (`self.IsHovered`)
        (set `local.tileColor` (`KismetMathLibrary.Conv_VectorToLinearColor` (* (`KismetMathLibrary.Conv_LinearColorToVector` (`local.tileColor`)) 3.0)))
        (`MeshComponent.SetScalarParameterValueOnMaterials` (`self.StaticMesh`) "bIsVisible" 1.0)))
    (:`then_8`
      (if (`self.bIsSpawnZone`)
        (set `local.tileColor` (struct :`R` 0.132812 :`G` 0.796875 :`B` 0.208846 :`A` 1.0))
        (`MeshComponent.SetScalarParameterValueOnMaterials` (`self.StaticMesh`) "bIsVisible" 1.0)))
    (:`then_9`
      ;[1 1 1] Temp: When both PassThroughDamage and StoodOnDamage values are higher than 0, the damage tiles will be marked as red
      (if (and (> (`self.PassThroughDamage`) 0) (> (`self.StoodOnDamage`) 0))
        (set `local.tileColor` (struct :`R` 0.34375 :`B` 0.020861 :`A` 1.0))
        (`MeshComponent.SetScalarParameterValueOnMaterials` (`self.StaticMesh`) "bIsVisible" 1.0)))
    (:`then_10`
      (`MeshComponent.SetVectorParameterValueOnMaterials` (`self.StaticMesh`) "TileColor" (`KismetMathLibrary.Conv_LinearColorToVector` (`local.tileColor`))))))

(fn `SetTileSize`
  (bind _staticmesh (`self.StaticMesh`))
  (bind (_returnvalue_x _returnvalue_y) (`KismetMathLibrary.BreakVector` (* (`SceneComponent.K2_GetComponentScale` _staticmesh) (/ (`/Game/Blueprints/GridBPs/GridObjects/BP_Grid.TileSize` (`self.Grid`)) 50.0))))
  (`SceneComponent.SetWorldScale3D` _staticmesh (`KismetMathLibrary.MakeVector` _returnvalue_x _returnvalue_y 0.01)))

(fn `SetWidgetVariables`
  (bind _asw_grid_tile_info (cast `/Game/Blueprints/UI_Widgets/Combat/Grid/W_GridTileInfo` (`WidgetComponent.GetUserWidgetObject` (`self.Widget`)) :!pure true))
  (set `/Game/Blueprints/UI_Widgets/Combat/Grid/W_GridTileInfo.grid` (`self.Grid`) _asw_grid_tile_info)
  (set `/Game/Blueprints/UI_Widgets/Combat/Grid/W_GridTileInfo.gridIndex` (`self.GridIndex`) _asw_grid_tile_info))

(fn `UserConstructionScript`)