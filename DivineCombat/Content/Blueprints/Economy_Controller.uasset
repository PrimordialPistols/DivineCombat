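; Economy controller Blueprint that tracks the player's Renown as a simple counter.
; Renown resets to zero on BeginPlay, and the R and T keys raise or lower it by one.
; Tick prints the current value to screen every frame, which serves as a debug readout.
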(event `self.ReceiveBeginPlay`
  ;[1 1 1] Sets the player's Renown to 0 at the start of the game
  (bind _output_get (set `self.Renown` 0)))

(event `self.ReceiveTick`
  (params (DeltaSeconds :type "Float (single-precision)"))
  (`KismetSystemLibrary.PrintString` (`KismetTextLibrary.Conv_TextToString` (`KismetTextLibrary.Conv_IntToText` (`self.Renown`)))))

(event `Key|R`
  (params (Key :type "Key Structure"))
  (:`Pressed`
    (set `self.Renown` (+ (stale `self.ReceiveBeginPlay` _output_get) 1))))

(event `Key|T`
  (params (Key :type "Key Structure"))
  (:`Pressed`
    (set `self.Renown` (- (stale `self.ReceiveBeginPlay` _output_get) 1))))

(fn `UserConstructionScript`)