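; BaseEnemy_BP is a base enemy Blueprint that shows a health bar when the player's TopDownCharacter is nearby.
; BeginPlay caches the AI_HealthWidget from its widget component, and overlap events on a Sphere toggle that component's visibility.
; Tick writes Health to the widget from a newly made AIStatHolder struct fixed at full health, so the bar does not track damage.
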(event `self.ReceiveBeginPlay`
  ;[1 1 1] Displays Health Widget on AI
  (bind _asai_health_widget (cast `/Game/AI/AI_Blueprints/AI_HealthWidget` (`WidgetComponent.GetUserWidgetObject` (`self.HealthWidget`))))
  (set `self.HealthWidgetRef` _asai_health_widget))

(event `self.ReceiveTick`
  (params (DeltaSeconds :type "Float (single-precision)"))
  ;[1 1 1] Sets Health in Widget
  (set `/Game/AI/AI_Blueprints/AI_HealthWidget.Health` (`.CurrentHealth` (break `AIStatHolder` (make `AIStatHolder` 100.0))) (`self.HealthWidgetRef`)))

(event `self.Sphere.OnComponentBeginOverlap`
  (params (OverlappedComponent :type "PrimitiveComponent Object Reference") (OtherActor :type "Actor Object Reference") (OtherComp :type "PrimitiveComponent Object Reference") (OtherBodyIndex :type Integer) (bFromSweep :type Boolean) (SweepResult :type "HitResult Structure (by ref)"))
  ;[1 1 1] Shows Health bar when player is close to enemy
  (cast `/Game/TopDownBP/Blueprints/TopDownCharacter` OtherActor)
  (`SceneComponent.SetVisibility` (`self.HealthWidget`) true false))

(event `self.Sphere.OnComponentEndOverlap`
  (params (OverlappedComponent :type "PrimitiveComponent Object Reference") (OtherActor :type "Actor Object Reference") (OtherComp :type "PrimitiveComponent Object Reference") (OtherBodyIndex :type Integer))
  ;[1 1 1] Shows Health bar when player is close to enemy
  (cast `/Game/TopDownBP/Blueprints/TopDownCharacter` OtherActor)
  (`SceneComponent.SetVisibility` (`self.HealthWidget`) false false))

(fn `UserConstructionScript`)