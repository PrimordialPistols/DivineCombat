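; Turn-system Blueprint, named as a game mode, that sets up grid-based combat when play begins.
; It creates the combat screen widget and hands it the grid, the player controller and a list of all units ordered player faction first.
; It also tallies starting allied and enemy units on the grid.
; Sorting is a simple two-faction split, with an unused insertion sort left unconnected.
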(event `self.ReceiveBeginPlay`
  (bind _grid (`self.grid`))
  (bind _grid_2 (`self.grid`))
  (bind _returnvalue (`|CreateWidget` "/Game/Blueprints/Controllers/W_CombatScreen.W_CombatScreen_C"))
  (bind _output_get (set `self.CombatScreen` _returnvalue))
  (`UserWidget.AddToPlayerScreen` _output_get 0)
  ;[1 1 1] Get Local Reference to Grid
  (bind _outactors (`GameplayStatics.GetAllActorsOfClass` "/Game/Blueprints/Grid/BP_Grid.BP_Grid_C"))
  (bind _output_get_2 (set `self.grid` (`|GetArrayItem` _outactors)))
  (set `/Game/Blueprints/Controllers/W_CombatScreen.grid` _output_get_2 (`self.CombatScreen`))
  ;[1 1 1] Create Unit List
  (bind _outactors_2 (`GameplayStatics.GetAllActorsOfClass` "/Game/Blueprints/Controllers/BP_Unit.BP_Unit_C"))
  (bind _sortedunits (`self.SortUnitListByFaction` _outactors_2)) ; Currently only works for two factions, player and other
  (bind _output_get_3 (set `/Game/Blueprints/Controllers/W_CombatScreen.UnitList` _sortedunits (`self.CombatScreen`)))
  (for _array_element _output_get_3
    (if (`|EnumEquality` (`/Game/Blueprints/Controllers/BP_Unit.UnitFaction` _array_element) "NewEnumerator0")
      (set `/Game/Blueprints/Grid/BP_Grid.StartingAlliedUnits` (+ (`/Game/Blueprints/Grid/BP_Grid.StartingAlliedUnits` _grid_2) 1) _grid_2)
      (else
        (set `/Game/Blueprints/Grid/BP_Grid.StartingEnemyUnits` (+ (`/Game/Blueprints/Grid/BP_Grid.StartingEnemyUnits` _grid) 1) _grid))))
  ;[1 1 1] Get Local Reference to HUD widget and PlayerController
  (set `/Game/Blueprints/Controllers/W_CombatScreen.Player` (cast `/Game/Blueprints/Controllers/BP_PlayerController` (`GameplayStatics.GetPlayerController` 0) :!pure true) (`self.CombatScreen`)))

(fn `SortUnitListByFaction`
  (params (unsortedUnits :type "Array of /Game/Blueprints/Controllers/BP_Unit Object Reference"))
  (returns (sortedUnits :type "Array of /Game/Blueprints/Controllers/BP_Unit Object Reference"))
  (locals (sortingList :type "Array of /Game/Blueprints/Controllers/BP_Unit Object Reference") (currentTarget :type "/Game/Blueprints/Controllers/BP_Unit Object Reference") (currentTargetStepper :type Integer :default 1) (currentTargetFaction :type Integer :default 0) (playerFacList :type "Array of /Game/Blueprints/Controllers/BP_Unit Object Reference") (enemyFacList :type "Array of /Game/Blueprints/Controllers/BP_Unit Object Reference"))
  (for _array_element unsortedUnits
    (if (`|EnumEquality` (`/Game/Blueprints/Controllers/BP_Unit.UnitFaction` _array_element) "NewEnumerator0")
      (`KismetArrayLibrary.Array_Add` (`local.playerFacList`) _array_element)
      (else
        (`KismetArrayLibrary.Array_Add` (`local.enemyFacList`) _array_element))))
  (for _array_element_2 (`local.enemyFacList`)
    (`KismetArrayLibrary.Array_Add` (`local.playerFacList`) _array_element_2))
  (return (`local.playerFacList`)))

(fn `UserConstructionScript`)